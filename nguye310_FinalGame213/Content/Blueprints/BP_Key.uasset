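; BP_Key is an interactable key pickup linked to two portals.
; On Interact, it calls PickUpKeyMessage on both referenced portals, then destroys itself.
; The construction script creates a dynamic instance of MI_KeyMat on the Sphere and applies the key's Color variable to it.
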(event EventInteract
  (Class|BPIPortals|PickUpKey(Message) (Variables|Default|GetPortal))
  (Class|BPIPortals|PickUpKey(Message) (Variables|Default|GetPortal1))
  (Actor|DestroyActor))

(fn ConstructionScript
  (bind _sphere (Variables|Default|GetSphere))
  ;[1 1 1] Dynamic Material Setting
  (bind _returnvalue (Rendering|Material|CreateDynamicMaterialInstance _sphere 0 "/Game/Materials/GlowingMats/MI_KeyMat.MI_KeyMat" "None" :!class /Script/Engine.PrimitiveComponent))
  (Rendering|Material|SetVectorParameterValue _returnvalue "Color" (Variables|Default|GetColor) :!class /Script/Engine.MaterialInstanceDynamic)
  (Rendering|Material|SetMaterial _sphere 0 _returnvalue))