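; BP_myKart is a kart actor that moves itself along a spline path in the level.
; On BeginPlay it finds a BP_myKartPath actor, caches its spline length and starts a timeline.
; Each timeline update lerps the movement track across that length and sets the kart's transform from the spline, using world-space location and local-space rotation.
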(event Custom|playMyKartTimeline
  (bind _mykartmovement (Timeline|myKartTimeline Play)
    (:Update
      (Transformation|SetActorTransform (Math|Transform|MakeTransform (Spline|GetLocationatDistanceAlongSpline (Variables|/Game/Blueprints/BP_myKartPath.BP_myKartPath_C|GetSpline (Variables|Default|GetmyKartPathReference)) (Math|Float|Lerp 0.0 (Variables|Default|GetmyKartPathLength) _mykartmovement) "World") (Spline|GetRotationatDistanceAlongSpline (Variables|/Game/Blueprints/BP_myKartPath.BP_myKartPath_C|GetSpline (Variables|Default|GetmyKartPathReference)) (Math|Float|Lerp 0.0 (Variables|Default|GetmyKartPathLength) _mykartmovement) "Local") "1.000000,1.000000,1.000000")))))

(event EventBeginPlay
  ;[1 1 1] get reference external
  (bind _returnvalue (Actor|GetActorOfClass "/Game/Blueprints/BP_myKartPath.BP_myKartPath_C"))
  (Variables|Default|SetmyKartPathReference _returnvalue)
  ;[1 1 1] set spline length
  (Variables|Default|SetmyKartPathLength (Spline|GetSplineLength (Variables|/Game/Blueprints/BP_myKartPath.BP_myKartPath_C|GetSpline (Variables|Default|GetmyKartPathReference))))
  (CallFunction|PlayMyKartTimeline))

(fn ConstructionScript)