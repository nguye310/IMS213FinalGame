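; QuestDescription is a quest actor that gates a key behind portal activations.
; On BeginPlay it hides the referenced Key's sphere and text render components.
; Each ActivatePortal event increments a counter; when it reaches the maximum, the actor makes both Key components visible again and destroys itself.
; Only visibility is toggled on the Key, with no collision changes.
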(event Custom|ActivatePortal
  (Math|Integer|IncrementInt (Variables|Default|GetcurrentPortalActivated)
    (:%20%20
      (if (>= (Variables|Default|GetcurrentPortalActivated) (Variables|Default|GetmaxPortalActivated))
        ;[1 1 1] Make the key visible again
        (Rendering|SetVisibility (Variables|/Game/Blueprints/BP_Key.BP_Key_C|GetSphere (Variables|Default|GetKey)) true false)
        (Rendering|SetVisibility (Variables|/Game/Blueprints/BP_Key.BP_Key_C|GetTextRender (Variables|Default|GetKey)) true false)
        (Actor|DestroyActor)))))

(event EventBeginPlay
  (Rendering|SetVisibility (Variables|/Game/Blueprints/BP_Key.BP_Key_C|GetSphere (Variables|Default|GetKey)) false false)
  (Rendering|SetVisibility (Variables|/Game/Blueprints/BP_Key.BP_Key_C|GetTextRender (Variables|Default|GetKey)) false false))

(fn ConstructionScript)